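; TimerController is a Blueprint that times a run and records the best result in the "Check" CheckpointSave slot.
; Time starts at zero, or at the saved TimeSave when LoadSave is set, and accumulates on Tick while Flow is true.
; Overlapping TimerEnd stops Flow and overwrites TimeSave only if the new time is lower.
; The same TimeSave field serves as resume time and high score, and nothing here turns Flow on.
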(event `self.ReceiveTick`
  (params (DeltaSeconds :type "Float (single-precision)"))
  (if (`self.Flow`)
    (set `self.Time` (+ DeltaSeconds (`self.Time`)))))

(event `self.ReceiveBeginPlay`
  (bind _returnvalue (`GameplayStatics.DoesSaveGameExist` "Check"))
  (if _returnvalue
    (bind _returnvalue_2 (`GameplayStatics.LoadGameFromSlot` "Check"))
    (bind _ascheckpoint_save (cast `/Game/BP/Checkpoints/CheckpointSave` _returnvalue_2))
    (if (`/Game/BP/Checkpoints/CheckpointSave.Load_save` _ascheckpoint_save)
      (set `self.Time` (`/Game/BP/Checkpoints/CheckpointSave.Time_save` _ascheckpoint_save))
      (else
        (set `self.Time` 0.0)))
    (else
      (set `self.Time` 0.0))))

(event `self.TimerEnd.OnComponentBeginOverlap`
  (params (OverlappedComponent :type "PrimitiveComponent Object Reference") (OtherActor :type "Actor Object Reference") (OtherComp :type "PrimitiveComponent Object Reference") (OtherBodyIndex :type Integer) (bFromSweep :type Boolean) (SweepResult :type "HitResult Structure (by ref)"))
  (bind _time (`self.Time`))
  (set `self.Flow` false)
  (bind _returnvalue (`GameplayStatics.DoesSaveGameExist` "Check"))
  (if _returnvalue
    (bind _returnvalue_2 (`GameplayStatics.LoadGameFromSlot` "Check"))
    (bind _ascheckpoint_save (cast `/Game/BP/Checkpoints/CheckpointSave` _returnvalue_2))
    (if (< _time (`/Game/BP/Checkpoints/CheckpointSave.Time_save` _ascheckpoint_save))
      (set `/Game/BP/Checkpoints/CheckpointSave.Time_save` _time _ascheckpoint_save)
      (`GameplayStatics.SaveGameToSlot` _ascheckpoint_save "Check")
      (`KismetSystemLibrary.PrintString` "new high score"))
    (else
      (`KismetSystemLibrary.PrintString` "Error : save doesn't exist"))))

(fn `UserConstructionScript`)