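; DeathZone_BP is a death trigger volume that respawns the player at the last saved checkpoint.
; Any overlap on DeathTrigger disables player 0's input without checking the overlapping actor, then waits for DeathDelay.
; If a save exists in the LevelName slot, it restores the character's location and rotation from CheckpointSave and re-enables input.
; Without a save, it opens the level named by Level instead.
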(event `self.Death Trigger.OnComponentBeginOverlap`
  (params (OverlappedComponent :type "PrimitiveComponent Object Reference") (OtherActor :type "Actor Object Reference") (OtherComp :type "PrimitiveComponent Object Reference") (OtherBodyIndex :type Integer) (bFromSweep :type Boolean) (SweepResult :type "HitResult Structure (by ref)"))
  (bind _ascharacter (cast `/Game/BP/character` (`GameplayStatics.GetPlayerCharacter` 0)))
  (`self.DisableInput` _ascharacter (`GameplayStatics.GetPlayerController` 0))
  (`KismetSystemLibrary.Delay` (`self.DeathDelay`))
  (bind _returnvalue (`GameplayStatics.DoesSaveGameExist` (`self.Level Name`)))
  (if _returnvalue
    ;[1 1 1] Save Exist
    (bind _returnvalue_2 (`GameplayStatics.LoadGameFromSlot` (`self.Level Name`)))
    (bind _ascheckpoint_save (cast `/Game/BP/Checkpoints/CheckpointSave` _returnvalue_2))
    (bind _ascharacter_2 (cast `/Game/BP/character` (`GameplayStatics.GetPlayerCharacter` 0)))
    (`self.K2_SetActorLocation` _ascharacter_2 (`/Game/BP/Checkpoints/CheckpointSave.PlayerLocation_save` _ascheckpoint_save) false false)
    (`self.K2_SetActorRotation` _ascharacter_2 (`/Game/BP/Checkpoints/CheckpointSave.PlayerRotation_save` _ascheckpoint_save) false)
    (`self.EnableInput` _ascharacter_2 (`GameplayStatics.GetPlayerController` 0))
    (else
      ;[1 1 1] Save doesn't exist
      (`GameplayStatics.OpenLevel` (`self.Level`)))))

(fn `UserConstructionScript`)