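; Checkpoint actor that, when its trigger is overlapped, either saves the player's position or resets the saved checkpoint, depending on its Load flag.
; With Load on, it captures the player character's location and rotation and writes them with LoadSave set into a CheckpointSave slot named by LevelName, creating the save if needed.
; With Load off, it clears LoadSave in the existing save.
; Debug prints show the captured and re-read rotation.
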(event `self.Trigger.OnComponentBeginOverlap`
  (params (OverlappedComponent :type "PrimitiveComponent Object Reference") (OtherActor :type "Actor Object Reference") (OtherComp :type "PrimitiveComponent Object Reference") (OtherBodyIndex :type Integer) (bFromSweep :type Boolean) (SweepResult :type "HitResult Structure (by ref)"))
  (bind _playerlocation (`self.PlayerLocation`))
  (bind _level_name (`self.Level Name`))
  (bind _playerrotation (`self.PlayerRotation`))
  (if (`self.Load`)
    (`|ExecutionSequence`
      (:`then_0`
        ;[1 1 1] Get character position
        (bind _ascharacter (cast `/Game/BP/character` (`GameplayStatics.GetPlayerCharacter` 0)))
        (set `self.PlayerLocation` (`self.K2_GetActorLocation` _ascharacter))
        (bind _output_get (set `self.PlayerRotation` (`self.K2_GetActorRotation` _ascharacter)))
        (`KismetSystemLibrary.PrintString` (`KismetStringLibrary.Conv_RotatorToString` _output_get)))
      (:`then_1`
        ;[1 1 1] Save that position
        (bind _returnvalue (`GameplayStatics.DoesSaveGameExist` (`self.Level Name`)))
        (if _returnvalue
          (bind _returnvalue_2 (`GameplayStatics.LoadGameFromSlot` (`self.Level Name`)))
          (bind _ascheckpoint_save (cast `/Game/BP/Checkpoints/CheckpointSave` _returnvalue_2))
          (set `/Game/BP/Checkpoints/CheckpointSave.PlayerLocation_save` _playerlocation _ascheckpoint_save)
          (set `/Game/BP/Checkpoints/CheckpointSave.PlayerRotation_save` _playerrotation _ascheckpoint_save)
          (set `/Game/BP/Checkpoints/CheckpointSave.Load_save` true _ascheckpoint_save)
          (`GameplayStatics.SaveGameToSlot` _ascheckpoint_save _level_name)
          (bind _returnvalue_3 (`GameplayStatics.LoadGameFromSlot` (`self.Level Name`)))
          (bind _ascheckpoint_save_2 (cast `/Game/BP/Checkpoints/CheckpointSave` _returnvalue_3))
          (`KismetSystemLibrary.PrintString` (`KismetStringLibrary.Conv_RotatorToString` (`/Game/BP/Checkpoints/CheckpointSave.PlayerRotation_save` _ascheckpoint_save_2)) true true (struct :`R` 1.0 :`B` 0.094356 :`A` 1.0))
          (else
            (bind _returnvalue_4 (`GameplayStatics.CreateSaveGameObject` "/Game/BP/Checkpoints/CheckpointSave.CheckpointSave_C"))
            (set `/Game/BP/Checkpoints/CheckpointSave.PlayerLocation_save` _playerlocation _returnvalue_4)
            (set `/Game/BP/Checkpoints/CheckpointSave.PlayerRotation_save` _playerrotation _returnvalue_4)
            (set `/Game/BP/Checkpoints/CheckpointSave.Load_save` true _returnvalue_4)
            (`GameplayStatics.SaveGameToSlot` _returnvalue_4 _level_name)))))
    (else
      ;[1 1 1] Reset save
      (bind _returnvalue_5 (`GameplayStatics.LoadGameFromSlot` (`self.Level Name`)))
      (bind _ascheckpoint_save_3 (cast `/Game/BP/Checkpoints/CheckpointSave` _returnvalue_5))
      (set `/Game/BP/Checkpoints/CheckpointSave.Load_save` false _ascheckpoint_save_3)
      (`GameplayStatics.SaveGameToSlot` _ascheckpoint_save_3 (`self.Level Name`)))))

(fn `UserConstructionScript`)